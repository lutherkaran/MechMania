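; Base AI controller for enemies that runs a behavior tree and starts in a Passive state on possess.
; Perception updates are checked for sight, hearing and damage stimuli, each routed to its own handler.
; Handlers act only while Passive or Investigating: seeing the player or taking damage switches to Attacking, while noise switches to Investigating.
; State, attack target and point of interest are written to the Blackboard for the tree.
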(event `self.ReceivePossess`
  (params (PossessedPawn :type "Pawn Object Reference"))
  (`self.RunBehaviorTree` "/Game/Blueprints/AI/BT_Eneme_Base.BT_Eneme_Base")
  (`self.SetStateAsPassive`))

(event `self.AIPerception.OnPerceptionUpdated`
  (params (UpdatedActors :type "Array of Actor Object Reference (by ref)"))
  (for _array_element UpdatedActors
    (`|ExecutionSequence`
      (:`then_0`
        (bind _sensed (`self.CanSee` _array_element "NewEnumerator1"))
        (if _sensed
          (`self.HandleSensedSight` _array_element)))
      (:`then_1`
        (bind (_sensed_2 _stimulus) (`self.CanSee` _array_element "NewEnumerator2"))
        (if _sensed_2
          (`self.HandleSensedSound` (`.StimulusLocation` (break `AIStimulus` _stimulus)))))
      (:`then_2`
        (bind _sensed_3 (`self.CanSee` _array_element "NewEnumerator3"))
        (if _sensed_3
          (`self.HandSensedDamage` _array_element))))))

(fn `CanSee`
  (params (Actor :type "Actor Object Reference") (Sense :type "/Game/Blueprints/AI/Enums/E_AISense Enum" :default "NewEnumerator0"))
  (returns (Sensed :type Boolean) (Stimulus :type "AIStimulus Structure"))
  (bind _info (`AIPerceptionComponent.GetActorsPerception` (`self.AIPerception`) Actor))
  (for _array_element (`.LastSensedStimuli` (break `ActorPerceptionBlueprintInfo` _info))
    (bind _returnvalue (`AIPerceptionSystem.GetSenseClassForStimulus` _array_element))
    (if (== _returnvalue (select `/Game/Blueprints/AI/Enums/E_AISense` Sense :`NewEnumerator1` "/Script/AIModule.AISense_Sight" :`NewEnumerator2` "/Script/AIModule.AISense_Hearing" :`NewEnumerator3` "/Script/AIModule.AISense_Damage" :!type "Object Class Reference"))
      (return (`.bSuccessfullySensed` (break `AIStimulus` _array_element)) _array_element))))

(fn `GetCurrentState`
  (returns (State :type "/Game/Blueprints/AI/Enums/E_AIStates Enum"))
  (return (cast `/Game/Blueprints/AI/Enums/E_AIStates` (`BlackboardComponent.GetValueAsEnum` (`self.Blackboard`) (`self.AIStatesKeyName`)))))

(fn `HandleSensedSight`
  (params (Actor :type "Actor Object Reference"))
  (bind _state (`self.GetCurrentState`))
  (switch `/Game/Blueprints/AI/Enums/E_AIStates` _state
    (:`NewEnumerator0`
      _)
    (:`NewEnumerator2`
      _))
  (if (== Actor (`GameplayStatics.GetPlayerCharacter` 0))
    (`self.SetStateAsAttacking` Actor)))

(fn `HandleSensedSound`
  (params (Location :type "Vector Structure"))
  (bind _state (`self.GetCurrentState`))
  (switch `/Game/Blueprints/AI/Enums/E_AIStates` _state
    (:`NewEnumerator0`
      _)
    (:`NewEnumerator2`
      _))
  (`self.SetStateAsInvestigating` Location))

(fn `HandSensedDamage`
  (params (Actor :type "Actor Object Reference"))
  (bind _state (`self.GetCurrentState`))
  (switch `/Game/Blueprints/AI/Enums/E_AIStates` _state
    (:`NewEnumerator0`
      _)
    (:`NewEnumerator2`
      _))
  (`self.SetStateAsAttacking` Actor))

(fn `SetStateAsAttacking`
  (params (AttackTarget :type "Actor Object Reference"))
  (`BlackboardComponent.SetValueAsObject` (`self.Blackboard`) (`self.AttackTargetKeyName`) AttackTarget)
  (`BlackboardComponent.SetValueAsEnum` (`self.Blackboard`) (`self.AIStatesKeyName`) (enumliteral `/Game/Blueprints/AI/Enums/E_AIStates` "NewEnumerator1")))

(fn `SetStateAsInvestigating`
  (params (Location :type "Vector Structure"))
  (bind _blackboard (`self.Blackboard`))
  (`BlackboardComponent.SetValueAsEnum` _blackboard (`self.AIStatesKeyName`) (enumliteral `/Game/Blueprints/AI/Enums/E_AIStates` "NewEnumerator2"))
  (`BlackboardComponent.SetValueAsVector` _blackboard (`self.PointOfInterestKeyName`) Location))

(fn `SetStateAsPassive`
  (`BlackboardComponent.SetValueAsEnum` (`self.Blackboard`) (`self.AIStatesKeyName`) (enumliteral `/Game/Blueprints/AI/Enums/E_AIStates` "NewEnumerator0")))

(fn `UserConstructionScript`)